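; BP_PlayerCharacter is the player character, handling basic look and movement input.
; Mouse axes drive controller yaw and inverted pitch, scaled by separate horizontal and vertical rotation speeds.
; Movement axes feed AddMovementInput along the actor's forward and right vectors, scaled by MoveSpeed and world delta time.
; The axis named Move Vertical drives sideways strafing, and Tick is empty.
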(event `self.ReceiveTick`
  (params (DeltaSeconds :type "Float (single-precision)")))

(event `InputAxisKey|MouseY`
  (params (AxisValue :type "Float (single-precision)"))
  (`self.AddControllerPitchInput` (* AxisValue (`self.CameraVerticalRotationSpeed`) -1.0)))

(event `InputAxisKey|MouseX`
  (params (AxisValue :type "Float (single-precision)"))
  (`self.AddControllerYawInput` (* AxisValue (`self.CameraHorizontalRotationSpeed`))))

(event `InputAxis|Move Fowerd`
  (params (AxisValue :type "Float (single-precision)"))
  (`self.AddMovementInput` (`self.GetActorForwardVector`) (* AxisValue (`GameplayStatics.GetWorldDeltaSeconds`) (`self.MoveSpeed`))))

(event `InputAxis|Move Vertical`
  (params (AxisValue :type "Float (single-precision)"))
  (`self.AddMovementInput` (`self.GetActorRightVector`) (* AxisValue (`GameplayStatics.GetWorldDeltaSeconds`) (`self.MoveSpeed`))))

(fn `UserConstructionScript`)