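; BP_Floor is a floor actor that tiles a mesh into a rectangular grid.
; Its construction script adds one InstancedStaticMesh instance per cell of XCount by YCount, spaced by UnitWidth and UnitHeight, with shadow casting turned off.
; The event graph holds no active logic, so the grid is built entirely in the construction script.
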(fn `UserConstructionScript`
  (bind _instancedstaticmesh (`self.InstancedStaticMesh`))
  (set `self.OldXCount` (`self.XCount`))
  (set `self.OldYCount` (`self.YCount`))
  (for _index (range (`self.YCount`))
    (for _index_2 (range (`self.XCount`))
      (`InstancedStaticMeshComponent.AddInstance` _instancedstaticmesh (`KismetMathLibrary.Conv_VectorToTransform` (`KismetMathLibrary.MakeVector` (* _index_2 (`self.UnitWidth`)) (* _index (`self.UnitHeight`)))))
      (`PrimitiveComponent.SetCastShadow` _instancedstaticmesh false))))